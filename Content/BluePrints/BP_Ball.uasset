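; BP_Ball is a ball actor that moves in a straight line along its Direction variable at Speed.
; Each Tick, it adds the normalized Direction, scaled by Speed and DeltaSeconds, to the Sphere component's world location and sets that as the actor transform.
; Rotation and scale carry over from the Sphere, and the move is unswept.
; BeginPlay, overlap and construction logic are empty.
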(event `self.ReceiveTick`
  (params (DeltaSeconds :type "Float (single-precision)"))
  (`self.K2_SetActorTransform` (`KismetMathLibrary.MakeTransform` (+ (* (`KismetMathLibrary.Normal` (`self.Direction`)) (* DeltaSeconds (`self.Speed`))) (.location (`SceneComponent.K2_GetComponentToWorld` (`self.Sphere`)))) (.rotation (`SceneComponent.K2_GetComponentToWorld` (`self.Sphere`))) (.scale (`SceneComponent.K2_GetComponentToWorld` (`self.Sphere`))))))

(event `self.ReceiveActorBeginOverlap`
  (params (OtherActor :type "Actor Object Reference")))

(fn `UserConstructionScript`)