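; A simple AI character that wanders randomly around the navigable area.
; On BeginPlay it moves to a random reachable point within a wide radius of its location, then repeats on a looping timer whose interval is randomized once at start.
; A separate GoAccel event sets the character's max walk speed to a passed-in value.
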(event `self.ReceiveBeginPlay`
  (`self.AIMovement`)
  (`KismetSystemLibrary.K2_SetTimerDelegate` (delegate `AIMovement`) (`KismetMathLibrary.RandomFloatInRange` 2.0 5.0) true))

(event `AIMovement`
  (`|AIMoveTo` self (`NavigationSystemV1.K2_GetRandomLocationInNavigableRadius` (`self.K2_GetActorLocation`) 5000.0 null null) null))

(event `GoAccel`
  (params (`最大行走速度` :type "Float (double-precision)"))
  (set `CharacterMovementComponent.MaxWalkSpeed` `最大行走速度` (`self.CharacterMovement`)))

(fn `UserConstructionScript`)