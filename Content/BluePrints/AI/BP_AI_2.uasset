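; BP_AI_2 is an AI character that melee-attacks BP_Flandre when that actor overlaps its PunchField.
; Overlap starts a punch cycle that plays the FemalePunch montage, applies fixed damage immediately and sets a looping timer with the montage's length to repeat it.
; Ending the overlap clears that timer.
; A separate GoAccel event sets the character's maximum walk speed from its parameter.
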(event `loop`
  (bind _returnvalue (`AnimInstance.Montage_Play` (`SkeletalMeshComponent.GetAnimInstance` (`self.Mesh`)) "/Game/Characters/Animation/FemalePunch.FemalePunch" 1.0 "MontageLength" 0.0 true :!label _label))
  (bind _returnvalue_2 (`KismetSystemLibrary.K2_SetTimerDelegate` (delegate `loop`) _returnvalue true))
  (`GameplayStatics.ApplyDamage` (stale `self.PunchField.OnComponentBeginOverlap` _asbp_flandre) 10.0))

(event `self.PunchField.OnComponentBeginOverlap`
  (params (OverlappedComponent :type "PrimitiveComponent Object Reference") (OtherActor :type "Actor Object Reference") (OtherComp :type "PrimitiveComponent Object Reference") (OtherBodyIndex :type Integer) (bFromSweep :type Boolean) (SweepResult :type "HitResult Structure (by ref)"))
  (bind _asbp_flandre (cast `/Game/Characters/Flandre/BP_Flandre` OtherActor))
  (goto _label))

(event `self.PunchField.OnComponentEndOverlap`
  (params (OverlappedComponent :type "PrimitiveComponent Object Reference") (OtherActor :type "Actor Object Reference") (OtherComp :type "PrimitiveComponent Object Reference") (OtherBodyIndex :type Integer))
  (cast `/Game/Characters/Flandre/BP_Flandre` OtherActor)
  (`KismetSystemLibrary.K2_ClearAndInvalidateTimerHandle` (stale `loop` _returnvalue_2)))

(event `GoAccel`
  (params (`最大行走速度` :type "Float (double-precision)"))
  (set `CharacterMovementComponent.MaxWalkSpeed` `最大行走速度` (`self.CharacterMovement`)))

(fn `UserConstructionScript`)