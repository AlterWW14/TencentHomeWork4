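; BP_Lamp_Wall is an interactive wall lamp for a puzzle that moves a BP_Wall once every lamp is on.
; A box overlap with MyCharacter enables input and opens a gate, so E toggles the spotlight and Opened state only nearby.
; Switching on checks all lamp instances and calls RotateSelf on the first BP_Wall found if all are open.
; Switching any lamp off calls CloseSelf on that wall.
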(event `Key|E`
  (params (Key :type "Key Structure"))
  (:`Pressed`
    (`/Engine/EditorBlueprintResources/StandardMacros.Gate` true :!label _label
      (:`Exit`
        (`SceneComponent.ToggleVisibility` (`self.SpotLight`) false)
        (if (`self.bOpened`)
          (set `self.bOpened` false)
          (bind _outactors (`GameplayStatics.GetAllActorsOfClass` "/Game/BluePrints/BP_Wall.BP_Wall_C"))
          (`/Game/BluePrints/BP_Wall.CloseSelf` (`|GetArrayItem` _outactors))
          (else
            (set `self.bOpened` true)
            (bind _outactors_2 (`GameplayStatics.GetAllActorsOfClass` "BP_Lamp_Wall_C"))
            (set `self.Length` (`KismetArrayLibrary.Array_Length` _outactors_2))
            (for _array_element _outactors_2
              (if (`/Game/BluePrints/BP_Lamp_Wall.bOpened` _array_element)
                (set `self.Opened` (+ (`self.Opened`) 1))
                (else
                  (`KismetSystemLibrary.PrintString` "Hello")
                  (break))))
            (if (== (`self.Opened`) (`self.Length`))
              (set `self.Opened` 0)
              (bind _outactors_3 (`GameplayStatics.GetAllActorsOfClass` "/Game/BluePrints/BP_Wall.BP_Wall_C"))
              (`/Game/BluePrints/BP_Wall.RotateSelf` (`|GetArrayItem` _outactors_3))
              (else
                (set `self.Opened` 0)))))))))

(event `self.Box.OnComponentBeginOverlap`
  (params (OverlappedComponent :type "PrimitiveComponent Object Reference") (OtherActor :type "Actor Object Reference") (OtherComp :type "PrimitiveComponent Object Reference") (OtherBodyIndex :type Integer) (bFromSweep :type Boolean) (SweepResult :type "HitResult Structure (by ref)"))
  (cast `/Game/BluePrints/MyCharacter` OtherActor)
  (`self.EnableInput` (`GameplayStatics.GetPlayerController` 0))
  (goto _label :!via `Open`))

(event `self.Box.OnComponentEndOverlap`
  (params (OverlappedComponent :type "PrimitiveComponent Object Reference") (OtherActor :type "Actor Object Reference") (OtherComp :type "PrimitiveComponent Object Reference") (OtherBodyIndex :type Integer))
  (cast `/Game/BluePrints/MyCharacter` OtherActor)
  (`self.DisableInput` (`GameplayStatics.GetPlayerController` 0))
  (goto _label :!via `Close`))

(fn `UserConstructionScript`)